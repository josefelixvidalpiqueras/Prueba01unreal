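; BP_FinishLine is the runner game's finish line actor, which ends the run when the player character hits its static mesh.
; The hit event casts to BP_RunnerGameCharacter and compares TotalCoins with a hardcoded perfect score to show either a perfect-win or a regular win widget.
; Both branches then wait briefly and reopen the current level by name, restarting the run.
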(event OnComponentHit(StaticMesh)
  (params (HitComponent :type Primitive%20Component%20Object%20Reference) (OtherActor :type Actor%20Object%20Reference) (OtherComp :type Primitive%20Component%20Object%20Reference) (NormalImpulse :type Vector :default "0, 0, 0") (Hit :type Hit%20Result%20Structure%20%28by%20ref%29))
  ;[1 1 1] Evento de choque con la línea de meta que ejecuta un condicional para saber si el usuario ha hecho una puntuación perfecta o no y muestra el cartel de victoria en consecuencia.
  (bind _asbp_runner_game_character (Utilities|Casting|CastToBP_RunnerGameCharacter OtherActor))
  (if (== (Variables|/Game/RunnerGame/Blueprints/BP_RunnerGameCharacter.BP_RunnerGameCharacter_C|GetTotalCoins _asbp_runner_game_character) 23)
    (bind _returnvalue (UserInterface|CreateWidget "/Game/RunnerGame/Blueprints/UW_PerfectWin.UW_PerfectWin_C"))
    (UserInterface|Viewport|AddtoViewport _returnvalue 0)
    (Utilities|FlowControl|Delay 2.0)
    (bind _returnvalue_2 (Game|GetCurrentLevelName true))
    (Game|OpenLevel(byName) (Utilities|String|StringToName _returnvalue_2))
    (else
      (bind _returnvalue_3 (UserInterface|CreateWidget "/Game/RunnerGame/Blueprints/UW_Win.UW_Win_C"))
      (UserInterface|Viewport|AddtoViewport _returnvalue_3 0)
      (Utilities|FlowControl|Delay 2.0)
      (bind _returnvalue_4 (Game|GetCurrentLevelName true))
      (Game|OpenLevel(byName) (Utilities|String|StringToName _returnvalue_4)))))

(event EventBeginPlay)

(event Collision|EventActorBeginOverlap
  (params (OtherActor :type Actor%20Object%20Reference)))

(event EventTick
  (params (DeltaSeconds :type Float%20%28single-precision%29)))

(fn ConstructionScript)